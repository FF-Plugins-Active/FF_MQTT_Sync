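; Template actor that demonstrates a synchronous Paho MQTT client in Unreal.
; On BeginPlay it spawns an MQTT_Manager_Paho_Sync and connects over MQTT v5 using HiveMQ server and credentials from the GI_Plugins game instance.
; On a successful connection it binds arrived, delivered and lost delegates, publishes a test message and subscribes to a topic.
; Connection status, publish and subscribe results, and delegate events are printed on screen.
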(event `self.ReceiveBeginPlay`
  (bind _asgi_plugins (cast `/Game/Player/GI_Plugins` (`GameplayStatics.GetGameInstance`)))
  (set `self.REF_GI_Plugins` _asgi_plugins)
  (bind _returnvalue (`|SpawnActorFromClass` "/Script/FF_MQTT_Sync.MQTT_Manager_Paho_Sync" (`KismetMathLibrary.MakeTransform` (0.0 0.0 0.0)) "Undefined" "MultiplyWithRoot" null null))
  (bind _output_get (set `self.REF_Paho_Sync` _returnvalue))
  (`MQTT_Manager_Paho_Sync.MQTT_Sync_Init` _output_get (delegate `Delegate_Client`) (make `PahoClientParams_Sync` "UE5_Paho_C_Sync" (`BlueprintMapLibrary.Map_Find` (`/Game/Player/GI_Plugins.Servers` (`self.REF_GI_Plugins`)) "hivemq") (`BlueprintMapLibrary.Map_Find` (`/Game/Player/GI_Plugins.Users` (`self.REF_GI_Plugins`)) "hivemq") (`BlueprintMapLibrary.Map_Find` (`/Game/Player/GI_Plugins.Passwords` (`self.REF_GI_Plugins`)) "hivemq") "" "" "" "" "" "" 20 "V_5")))

(event `Delegate_Arrived_Event`
  (params (Out_Result :type "PahoArrived_Sync Structure"))
  (`KismetSystemLibrary.PrintString` (`KismetStringLibrary.Concat_StrStr` Out_Result_Message " = " Out_Result_TopicName) true true (struct :`G` 1.0 :`A` 1.0) 30.0))

(event `Delegate_Delivered_Event`
  (params (Out_Result :type String))
  (`KismetSystemLibrary.PrintString` Out_Result true true (struct :`G` 1.0 :`A` 1.0) 30.0))

(event `Delegate_Lost_Event`
  (params (Out_Cause :type String))
  (`KismetSystemLibrary.PrintString` Out_Cause true true (struct :`R` 1.0 :`A` 1.0) 30.0))

(event `Delegate_Client`
  (params (bIsSuccessfull :type Boolean) (Out_Code :type "JsonObjectWrapper Structure"))
  (bind _outvalue (`|GetJsonField` Out_Code "Description"))
  (`KismetSystemLibrary.PrintString` _outvalue true true (select `bool` bIsSuccessfull :`false` (struct :`R` 1.0 :`A` 1.0) :`true` (struct :`G` 1.0 :`A` 1.0) :!type "LinearColor Structure") 30.0)
  (if bIsSuccessfull
    (`|ExecutionSequence`
      (:`then_0`
        (add `MQTT_Manager_Paho_Sync.Delegate_Arrived` (`self.REF_Paho_Sync`) (delegate `Delegate_Arrived_Event`))
        (add `MQTT_Manager_Paho_Sync.Delegate_Delivered` (`self.REF_Paho_Sync`) (delegate `Delegate_Delivered_Event`))
        (add `MQTT_Manager_Paho_Sync.Delegate_Lost` (`self.REF_Paho_Sync`) (delegate `Delegate_Lost_Event`)))
      (:`then_1`
        (bind (_out_code _returnvalue) (`MQTT_Manager_Paho_Sync.MQTT_Sync_Publish` (`self.REF_Paho_Sync`) "ue5_sync" "this message sent from ue5" "QoS_0" 0))
        (`KismetSystemLibrary.PrintString` (`KismetStringLibrary.Concat_StrStr` "publish state = " (`KismetStringLibrary.Conv_BoolToString` _returnvalue)) true true (select `bool` _returnvalue :`false` (struct :`R` 1.0 :`A` 1.0) :`true` (struct :`G` 1.0 :`A` 1.0) :!type "LinearColor Structure") 30.0)
        (bind (_out_code_2 _returnvalue_2) (`MQTT_Manager_Paho_Sync.MQTT_Sync_Subscribe` (`self.REF_Paho_Sync`) "web" "QoS_0"))
        (`KismetSystemLibrary.PrintString` (`KismetStringLibrary.Concat_StrStr` "subscribe state = " (`KismetStringLibrary.Conv_BoolToString` _returnvalue_2)) true true (select `bool` _returnvalue_2 :`false` (struct :`R` 1.0 :`A` 1.0) :`true` (struct :`G` 1.0 :`A` 1.0) :!type "LinearColor Structure") 30.0)))))

(fn `UserConstructionScript`)