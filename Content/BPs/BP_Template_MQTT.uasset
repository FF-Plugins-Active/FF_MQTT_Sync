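; Template Blueprint that opens an MQTT connection to a HiveMQ cloud broker on BeginPlay.
; It reads the broker credentials from the GI_Plugins game instance, spawns an MQTT_Manager_Paho actor and initializes it with a connection callback.
; The callback prints the JSON description in green or red, and on success binds arrived, delivered and lost delegates, whose handlers are empty stubs.
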(event `self.ReceiveBeginPlay`
  (bind _asgi_plugins (cast `/Game/Player/GI_Plugins` (`GameplayStatics.GetGameInstance`)))
  (set `self.REF_GI_Plugins` _asgi_plugins)
  (bind _returnvalue (`|SpawnActorFromClass` "/Script/FF_MQTT.MQTT_Manager_Paho" (`KismetMathLibrary.MakeTransform` (0.0 0.0 0.0)) "Undefined" "MultiplyWithRoot" null null))
  (bind _output_get (set `self.REF_Paho_Manager` _returnvalue))
  (`MQTT_Manager_Paho.MQTT_Init` _output_get (delegate `CustomEvent`) (`BlueprintMapLibrary.Map_Find` (`/Game/Player/GI_Plugins.Users` (`self.REF_GI_Plugins`)) "hivemq") (`BlueprintMapLibrary.Map_Find` (`/Game/Player/GI_Plugins.Passwords` (`self.REF_GI_Plugins`)) "hivemq") "UE5_Paho_C_Client" "1fd6d9d6a70f4db8b156a705ae198047.s1.eu.hivemq.cloud" 8883 20 false))

(event `CustomEvent`
  (params (bIsSuccessfull :type Boolean) (Out_Code :type "JsonObjectWrapper Structure"))
  (bind _outvalue (`|GetJsonField` Out_Code "Description"))
  (`KismetSystemLibrary.PrintString` _outvalue true true (select `bool` bIsSuccessfull :`false` (struct :`R` 1.0 :`A` 1.0) :`true` (struct :`G` 1.0 :`A` 1.0) :!type "LinearColor Structure") 30.0)
  (if bIsSuccessfull
    (add `MQTT_Manager_Paho.Delegate_Arrived` (`self.REF_Paho_Manager`) (delegate `Delegate_Arrived_Event`))
    (add `MQTT_Manager_Paho.Delegate_Delivered` (`self.REF_Paho_Manager`) (delegate `Delegate_Delivered_Event`))
    (add `MQTT_Manager_Paho.Delegate_Lost` (`self.REF_Paho_Manager`) (delegate `Delegate_Lost_Event`))))

(event `Delegate_Arrived_Event`
  (params (Out_Result :type "PahoArrived Structure")))

(event `Delegate_Delivered_Event`
  (params (Out_Result :type "PahoDelivered Structure")))

(event `Delegate_Lost_Event`
  (params (Out_Cause :type String)))

(fn `UserConstructionScript`)